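; Mudskipper enemy Blueprint that keeps turning to face the player's camera and can show a flexing animation.
; Each Tick eases only the yaw toward the camera with RInterpTo, then reassigns the mesh's anim class from the IsFlexing flag, which this graph never sets.
; Capsule overlaps only print the other component's name, and GetTargetActor exposes TargetPoint, which the look-at logic does not use.
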(event OnComponentBeginOverlap(Capsule)
  (params (OverlappedComponent :type Primitive%20Component%20Object%20Reference) (OtherActor :type Actor%20Object%20Reference) (OtherComp :type Primitive%20Component%20Object%20Reference) (OtherBodyIndex :type Integer) (bFromSweep :type Boolean) (SweepResult :type Hit%20Result%20Structure%20%28by%20ref%29))
  (Development|PrintString (Utilities|GetDisplayName OtherComp)))

(event OnComponentEndOverlap(Capsule)
  (params (OverlappedComponent :type Primitive%20Component%20Object%20Reference) (OtherActor :type Actor%20Object%20Reference) (OtherComp :type Primitive%20Component%20Object%20Reference) (OtherBodyIndex :type Integer)))

(event Custom|TargetActorLook
  (bind _self self)
  (bind _returnvalue (Transformation|GetActorRotation _self))
  (bind (_roll _pitch) (Math|Rotator|BreakRotator _returnvalue))
  (Transformation|SetActorRotation (Math|Rotator|MakeRotator _roll _pitch (.Yaw (Math|Rotator|BreakRotator (Math|Interpolation|RInterpTo _returnvalue (Math|Rotator|FindLookatRotation (Transformation|GetActorLocation _self) (Transformation|GetActorLocation (Game|GetPlayerCameraManager 0))) (Utilities|Time|GetWorldDeltaSeconds) 5.0))))))

(event EventBeginPlay)

(event Collision|EventActorBeginOverlap
  (params (OtherActor :type Actor%20Object%20Reference)))

(event EventTick
  (params (DeltaSeconds :type Float%20%28single-precision%29))
  (bind _mudskipper (Variables|Default|GetMudskipper))
  (CallFunction|TargetActorLook)
  (if (not (Variables|Default|GetIsFlexing))
    (Components|SkeletalMesh|SetAnimInstanceClass _mudskipper "/Game/Models/Animation_Blueprint/Mudskipper_animation.Mudskipper_animation_C")
    (else
      (Components|SkeletalMesh|SetAnimInstanceClass _mudskipper "/Game/Models/Animation_Blueprint/FlexingMudskipper_Animation.FlexingMudskipper_Animation_C"))))

(fn ConstructionScript)

(fn GetTargetActor
  (return (Variables|Default|GetTargetPoint)))
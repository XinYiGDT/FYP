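; Sulg enemy Blueprint that reacts to hits from boats and bullets and dies when its health runs out.
; Hit events match the hit component's name: "Boat" flip-flops IsHit on or off after a delay, while "Bullet" subtracts HP and sets IsDeth at zero or below.
; Tick polls IsDeth and destroys the actor after a short delay.
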(event EventTick
  (params (DeltaSeconds :type Float%20%28single-precision%29))
  (if (Variables|Default|GetIsDeth?)
    (Utilities|FlowControl|Delay 3.0)
    (Actor|DestroyActor)))

(event Collision|EventHit
  (params (MyComp :type Primitive%20Component%20Object%20Reference) (Other :type Actor%20Object%20Reference) (OtherComp :type Primitive%20Component%20Object%20Reference) (bSelfMoved :type Boolean) (HitLocation :type Vector :default "0, 0, 0") (HitNormal :type Vector :default "0, 0, 0") (NormalImpulse :type Vector :default "0, 0, 0") (Hit :type Hit%20Result%20Structure%20%28by%20ref%29))
  (bind _hitcomponent (Collision|BreakHitResult Hit))
  (bind _returnvalue (Utilities|GetObjectName _hitcomponent))
  (Utilities|FlowControl|Sequence
    (:then_0
      (if (Utilities|Enum|Equal(Enum) _returnvalue "Boat")
        (Utilities|FlowControl|FlipFlop
          (:A
            (Utilities|FlowControl|Delay 3.0)
            (Variables|Default|SetIsHit? true))
          (:B
            (Utilities|FlowControl|Delay 1.0)
            (Variables|Default|SetIsHit? false)))))
    (:then_1
      (if (Utilities|Enum|Equal(Enum) _returnvalue "Bullet")
        (bind _output_get (Variables|Default|SetHP (- (Variables|Default|GetHP) 10)))
        (if (<= _output_get 0)
          (Variables|Default|SetIsDeth? true))))))

(fn ConstructionScript)
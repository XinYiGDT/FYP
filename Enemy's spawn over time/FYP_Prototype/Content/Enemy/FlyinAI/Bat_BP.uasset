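; Flying bat enemy that loiters between random goal points, periodically swoops at a target or lands to fight on the ground, then takes off again.
; Tick drives a BehaviorSwich state, re-running the flight, pursuit or ground behavior tree every frame.
; Seven reached goals trigger a random dive or landing; distance checks and Delays time attacks and takeoff.
; Tick also offsets mesh and capsule per flight state and destroys the bat after death.
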(event Custom|PursuitPlayerFlying
  ;[1 1 1] PursuitPlayerFlug(Flying)
  (if (>= (Variables|Default|GetAttacCount) 7)
    (if (!= (Math|Random|RandomInteger 5) 0)
      (Variables|Default|SetGoal%20Bot (Variables|Default|GetTargetActorPoint))
      (Variables|Default|SetBehaviorSwich 1)
      (Variables|Default|SetAttacCount 0)
      (else
        ;;[1 1 1] Landing
        (if (not (Variables|Default|GetIsLanding))
          (Variables|Default|SetGoal%20Bot (Variables|Default|GetGroundActorPoint))
          (Variables|Default|SetIsLanding true)
          (Variables|Default|SetBehaviorSwich 1)
          (Variables|Default|SetAttacCount 0))))))

(event Custom|AdjustmentOfCollsion
  (bind _skeletalcomponent (Variables|Default|GetSkeletalComponent))
  (bind _skeletalcomponent_2 (Variables|Default|GetSkeletalComponent))
  ;[1 1 1] AdjustmentOfCollsion
  (if (Variables|Default|GetIsFlying)
    (Utilities|FlowControl|Sequence
      (:then_0
        (Transformation|SetWorldLocationAndRotation _skeletalcomponent (- (Transformation|GetWorldLocation (Variables|Default|GetCollisionComponent)) "0, 0,240.000000") (Transformation|GetWorldRotation _skeletalcomponent) false false))
      (:then_1
        (Transformation|SetWorldLocationAndRotation (Variables|Default|GetCapsule) (Transformation|GetWorldLocation (Variables|Default|GetCollisionComponent)) "-40.000000,0.000000, 0" false false)))
    (else
      (Utilities|FlowControl|Sequence
        (:then_0
          (Transformation|SetWorldLocationAndRotation _skeletalcomponent_2 (- (Transformation|GetWorldLocation (Variables|Default|GetCollisionComponent)) "0, 0,60.000000") (Transformation|GetWorldRotation _skeletalcomponent_2) false false))
        (:then_1
          (Transformation|SetWorldLocationAndRotation (Variables|Default|GetCapsule) (Transformation|GetWorldLocation (Variables|Default|GetCollisionComponent)) "-90.000000, 0, 0" false false))))))

(event Custom|ChangeBehavior
  ;[1 1 1] ChangeBehavior
  (switch int (Variables|Default|GetBehaviorSwich)
    (:0
      (bind _output_get (Variables|Default|SetBehavior%20To%20Run "/Game/Enemy/FlyinAI/BehaviorTree/Flight_BT.Flight_BT"))
      (bind _asaicontroller (Utilities|Casting|CastToAIController (Pawn|GetController)))
      (AI|RunBehaviorTree _asaicontroller _output_get)
      (Variables|Default|SetIsFlying true))
    (:1
      (bind _output_get_2 (Variables|Default|SetBehavior%20To%20Run "/Game/Enemy/FlyinAI/BehaviorTree/HotPursuit_BT.HotPursuit_BT"))
      (bind _asaicontroller_2 (Utilities|Casting|CastToAIController (Pawn|GetController)))
      (AI|RunBehaviorTree _asaicontroller_2 _output_get_2)
      (Variables|Default|SetIsFlying true))
    (:2
      (bind _output_get_3 (Variables|Default|SetBehavior%20To%20Run "/Game/Enemy/FlyinAI/BehaviorTree/Bat_BT.Bat_BT"))
      (bind _asaicontroller_3 (Utilities|Casting|CastToAIController (Pawn|GetController)))
      (AI|RunBehaviorTree _asaicontroller_3 _output_get_3)
      (Variables|Default|SetIsFlying false))))

(event Custom|Loitering
  (bind _goalpointactor (Variables|Default|GetGoalPointActor))
  (bind _nowindex (Variables|Default|GetNowIndex))
  (bind _output (Utilities|Array|Get(acopy) _goalpointactor _nowindex))
  ;[1 1 1] Loitering
  (if (Variables|Default|GetIsGoalReached)
    (Utilities|FlowControl|Sequence :!label _label
      (:then_0
        (Variables|Default|SetBackGoalActor (Variables|Default|GetNextGoalActor))
        (Variables|Default|SetIsGoalReached false)
        (Variables|Default|SetAttacCount (+ (Variables|Default|GetAttacCount) 1)))
      (:then_1
        (CallFunction|GetRound 0 (Utilities|Array|LastIndex _goalpointactor))
        (if (!= _output (Variables|Default|GetNextGoalActor))
          (Variables|Default|SetNextGoalActor _output)
          (else
            (goto _label)))))))

(event Custom|GetRound
  (params (MIn :type Integer) (Max :type Integer))
  ;[1 1 1] Get Round
  (Variables|Default|SetNowIndex (Math|Random|RandomIntegerinRange MIn Max)))

(event Custom|PursuitPlayerLanding
  (bind _groundactorpoint (Variables|Default|GetGroundActorPoint))
  ;[1 1 1] PursuitPlayerFlug(Landing)
  (if (== (Variables|Default|GetGoal%20Bot) _groundactorpoint)
    (if (Variables|Default|GetIsLanding)
      (if (< (Math|Vector|VectorLength (- (Transformation|GetActorLocation) (Transformation|GetActorLocation _groundactorpoint))) 6e+01)
        (Variables|Default|SetGoal%20Bot (Variables|Default|GetTargetActorPoint))
        (Variables|Default|SetBehaviorSwich 2)))))

(event Custom|FindLookAtRotation
  (bind _self self)
  (bind _returnvalue (Transformation|GetActorRotation _self))
  (bind (_roll _pitch) (Math|Rotator|BreakRotator _returnvalue))
  (if (== (Variables|Default|GetGoal%20Bot) (Variables|Default|GetTargetActorPoint))
    (if (== (Variables|Default|GetBehaviorSwich) 2)
      (Transformation|SetActorRotation (Math|Rotator|MakeRotator _roll _pitch (.Yaw (Math|Rotator|BreakRotator (Math|Interpolation|RInterpTo _returnvalue (Math|Rotator|FindLookatRotation (Transformation|GetActorLocation _self) (Transformation|GetActorLocation)) (Utilities|Time|GetWorldDeltaSeconds) 5.0))))))))

(event Custom|AttackJage
  (bind _goal_bot (Variables|Default|GetGoal%20Bot))
  (bind _goal_bot_2 (Variables|Default|GetGoal%20Bot))
  ;[1 1 1] AttackJage
  (if (Variables|Default|GetIsFlying)
    ;;[1 1 1] Flying
    (if (== (Variables|Default|GetBehaviorSwich) 1)
      (if (== _goal_bot_2 (Variables|Default|GetTargetActorPoint))
        (if (not (Variables|Default|GetIsAttacking))
          (if (< (Math|Vector|VectorLength (- (Transformation|GetActorLocation _goal_bot_2) (Transformation|GetActorLocation))) 1.3e+02)
            (Variables|Default|SetIsAttacking true)
            (Utilities|FlowControl|Delay 3.2)
            (Variables|Default|SetIsAttacking false)
            (else
              (Utilities|FlowControl|Delay 3e+01)))
          (Variables|Default|SetBehaviorSwich 0))))
    (else
      ;;[1 1 1] Not Flying
      (if (== (Variables|Default|GetBehaviorSwich) 2)
        (if (== _goal_bot (Variables|Default|GetTargetActorPoint))
          (if (< (Math|Vector|VectorLength (- (Transformation|GetActorLocation _goal_bot) (Transformation|GetActorLocation))) 2e+02)
            (Utilities|FlowControl|FlipFlop
              (:A
                (Utilities|FlowControl|Delay 3.0)
                (Variables|Default|SetIsAttacking true))
              (:B
                (Utilities|FlowControl|Delay 1.0)
                (Variables|Default|SetIsAttacking false)))))))))

(event Custom|TakeOff
  ;[1 1 1] TikeOff
  (if (Variables|Default|GetIsLanding)
    (Utilities|FlowControl|Delay 3e+01)
    (Variables|Default|SetIsLanding false)
    (Variables|Default|SetBehaviorSwich 0)))

(event EventBeginPlay
  (Utilities|FlowControl|Delay (Variables|Default|GetWake%20Up%20Delay))
  (if (not (Variables|Default|GetBT%20Initialized))
    (bind _asaicontroller (Utilities|Casting|CastToAIController (Pawn|GetController)))
    (AI|RunBehaviorTree _asaicontroller (Variables|Default|GetBehavior%20To%20Run))
    (Variables|Default|SetBT%20Initialized true)))

(event EventTick
  (params (DeltaSeconds :type Float%20%28single-precision%29))
  (if (not (Variables|Default|GetisDead))
    (CallFunction|ChangeBehavior)
    (CallFunction|Loitering)
    (CallFunction|AdjustmentOfCollsion)
    (CallFunction|PursuitPlayerFlying)
    (CallFunction|PursuitPlayerLanding)
    (CallFunction|FindLookatRotation)
    (CallFunction|TakeOff)
    (CallFunction|AttackJage)
    (if (<= (Variables|Default|GetHP) 0)
      (Variables|Default|SetisDead true))
    (else
      (Utilities|FlowControl|Delay 3.0)
      (Actor|DestroyActor))))

(event EventAddMovementInputCustom
  (params (WorldDirection :type Vector :default "0, 0, 0") (ScaleValue :type Float%20%28single-precision%29))
  (bind _returnvalue (Math|Rotator|MakeRotfromX WorldDirection))
  (bind (_roll _pitch _yaw) (Math|Rotator|BreakRotator _returnvalue))
  (Transformation|SetActorRotation (Math|Interpolation|RInterpTo (Transformation|GetActorRotation) (Math|Rotator|MakeRotator (Math|Float|Clamp(Float) _roll -1e+01 1e+01) (Math|Float|Clamp(Float) _pitch -1e+01 1e+01) _yaw) (Utilities|Time|GetWorldDeltaSeconds) 1.0))
  (Pawn|Input|AddMovementInput WorldDirection (* ScaleValue (Variables|Default|GetBot%20Speed%20Scale)) false))

(fn ConstructionScript)

(fn GetGoalActor
  (return (select (Variables|Default|GetIsGoalReached) (Variables|Default|GetNextGoalActor) (Variables|Default|GetBackGoalActor))))

(fn GetGoalBot
  (return (Variables|Default|GetGoal%20Bot)))

(fn OnGoalReached
  (bind _goal_cooldown_time (Variables|Default|GetGoal%20Cooldown%20Time))
  (Utilities|IsValid (Variables|Default|GetNextGoalActor)
    (:Is%20Valid
      (Variables|Default|SetIsGoalReached (not (Variables|Default|GetIsGoalReached)))
      (return _goal_cooldown_time true))
    (:Is%20Not%20Valid
      (return _goal_cooldown_time false))))
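; Cacoon is a physics-driven enemy object, tethered by a cable and physics constraint, that can be brought down by a projectile.
; On BeginPlay it receives an impulse with a random Y strength and random sign to start it moving.
; A hit from an actor whose display name matches Projectile makes the constraint linearly breakable, then releases the cable end and destroys the actor after delays.
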(event OnComponentHit(Cacoon)
  (params (HitComponent :type Primitive%20Component%20Object%20Reference) (OtherActor :type Actor%20Object%20Reference) (OtherComp :type Primitive%20Component%20Object%20Reference) (NormalImpulse :type Vector :default "0, 0, 0") (Hit :type Hit%20Result%20Structure%20%28by%20ref%29))
  (if (Utilities|Enum|Equal(Enum) (Utilities|GetDisplayName (.HitActor (Collision|BreakHitResult Hit))) (Utilities|GetDisplayName (Variables|Default|GetProjectile)))
    (Class|PhysicsConstraintComponent|SetLinearBreakable (Variables|Default|GetPhysicsConstraint) true 3e+01)
    (Utilities|FlowControl|Delay 1.0)
    (Variables|/Script/CableComponent.CableComponent|SetbAttachEnd (Variables|Default|GetCable) false)
    (Utilities|FlowControl|Delay 3.0)
    (Actor|DestroyActor)))

(event EventBeginPlay
  (bind _output_get (Variables|Default|SetPhysicsPower (Math|Vector|MakeVector (.X (Math|Vector|BreakVector (Variables|Default|GetPhysicsPower))) (Math|Random|RandomFloatinRange 1e+04 1.3e+04) (.Z (Math|Vector|BreakVector (Variables|Default|GetPhysicsPower))))))
  (if (== (Math|Random|RandomInteger 2) 0)
    (Variables|Default|SetPhysicsPower (Math|Vector|MakeVector (.X (Math|Vector|BreakVector _output_get)) (* (.Y (Math|Vector|BreakVector _output_get)) -1.0) (.Z (Math|Vector|BreakVector _output_get)))))
  (Physics|AddImpulse (Variables|Default|GetCacoon) (Variables|Default|GetPhysicsPower) "None" false))

(event Collision|EventActorBeginOverlap
  (params (OtherActor :type Actor%20Object%20Reference)))

(fn ConstructionScript)
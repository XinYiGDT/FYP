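; Bat_BP is a flying AI bot that travels toward goal actors under behavior tree control.
; After a wake-up delay on BeginPlay, it starts its behavior tree once through its AIController.
; Custom movement input smoothly rotates it toward the travel direction with clamped pitch and roll, then applies speed-scaled movement.
; Goal functions expose the target actor or bot, flip between two goal actors when the second is valid, and return a cooldown.
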(event EventBeginPlay
  (Utilities|FlowControl|Delay (Variables|Default|GetWake%20Up%20Delay))
  (if (not (Variables|Default|GetBT%20Initialized))
    (bind _asaicontroller (Utilities|Casting|CastToAIController (Pawn|GetController)))
    (AI|RunBehaviorTree _asaicontroller (Variables|Default|GetBehavior%20To%20Run))
    (Variables|Default|SetBT%20Initialized true)))

(event EventAddMovementInputCustom
  (params (WorldDirection :type Vector :default "0, 0, 0") (ScaleValue :type Float%20%28single-precision%29))
  (bind _returnvalue (Math|Rotator|MakeRotfromX WorldDirection))
  (bind (_roll _pitch _yaw) (Math|Rotator|BreakRotator _returnvalue))
  (Transformation|SetActorRotation (Math|Interpolation|RInterpTo (Transformation|GetActorRotation) (Math|Rotator|MakeRotator (Math|Float|Clamp(Float) _roll -3e+01 3e+01) (Math|Float|Clamp(Float) _pitch -3e+01 3e+01) _yaw) (Utilities|Time|GetWorldDeltaSeconds) 3.0))
  (Pawn|Input|AddMovementInput WorldDirection (* ScaleValue (Variables|Default|GetBot%20Speed%20Scale)) false))

(event EventCallTriggerActor)

(event EventCallTriggerActorEndOverlap)

(fn ConstructionScript)

(fn GetGoalActor
  (return (select (Variables|Default|GetIsGoalFlipped) (Variables|Default|GetGoalActorFlip) (Variables|Default|GetGoalActor))))

(fn GetGoalBot
  (return (Variables|Default|GetGoal%20Bot)))

(fn OnGoalReached
  (bind _goal_cooldown_time (Variables|Default|GetGoal%20Cooldown%20Time))
  (Utilities|IsValid (Variables|Default|GetGoalActorFlip)
    (:Is%20Valid
      (Variables|Default|SetIsGoalFlipped (not (Variables|Default|GetIsGoalFlipped)))
      (return _goal_cooldown_time true))
    (:Is%20Not%20Valid
      (return _goal_cooldown_time false))))
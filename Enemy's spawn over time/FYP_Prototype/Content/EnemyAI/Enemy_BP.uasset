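; Enemy actor Blueprint that reacts to hits involving a component named "Boat" and removes itself once flagged dead.
; Matching hits run a FlipFlop that alternates between setting IsHit true and clearing it, each after its own delay.
; Tick polls IsDeth, which is not set in this graph, and destroys the actor after a short delay when it is true.
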(event EventTick
  (params (DeltaSeconds :type Float%20%28single-precision%29))
  (if (Variables|Default|GetIsDeth?)
    (Utilities|FlowControl|Delay 3.0)
    (Actor|DestroyActor)))

(event Collision|EventHit
  (params (MyComp :type Primitive%20Component%20Object%20Reference) (Other :type Actor%20Object%20Reference) (OtherComp :type Primitive%20Component%20Object%20Reference) (bSelfMoved :type Boolean) (HitLocation :type Vector :default "0, 0, 0") (HitNormal :type Vector :default "0, 0, 0") (NormalImpulse :type Vector :default "0, 0, 0") (Hit :type Hit%20Result%20Structure%20%28by%20ref%29))
  (if (Utilities|Enum|Equal(Enum) (Utilities|GetObjectName (.HitComponent (Collision|BreakHitResult Hit))) "Boat")
    (Utilities|FlowControl|FlipFlop
      (:A
        (Utilities|FlowControl|Delay 3.0)
        (Variables|Default|SetIsHit? true))
      (:B
        (Utilities|FlowControl|Delay 1.0)
        (Variables|Default|SetIsHit? false)))))

(fn ConstructionScript)